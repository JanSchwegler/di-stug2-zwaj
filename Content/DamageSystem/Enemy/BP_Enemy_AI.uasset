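; BP_Enemy_AI is an enemy character that chases the player and attacks on arrival.
; PawnSensing's OnSeePawn sets IsSeeingPlayer, without checking which pawn was seen, and calls FollowPlayer, which runs AIMoveTo toward player character 0.
; On a successful move, a CanAttack gate clears itself and calls PlayAnimMontage, with no montage asset shown.
; Nothing here resets CanAttack or IsSeeingPlayer.
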(event OnSeePawn(PawnSensing)
  (params (Pawn :type Pawn%20Object%20Reference))
  (Variables|Default|SetisSeeingPlayer? true)
  (CallFunction|FollowPlayer))

(event Custom|FollowPlayer
  (if (Variables|Default|GetisSeeingPlayer?)
    (AI|AIMoveTo self "0, 0, 0" (Game|GetPlayerCharacter 0) 1e+02 false
      (:OnSuccess
        (if (Variables|Default|GetcanAttack?)
          (Variables|Default|SetcanAttack? false)
          (Animation|PlayAnimMontage 0 1.0 "None"))))))

(event EventBeginPlay)

(event Collision|EventActorBeginOverlap
  (params (OtherActor :type Actor%20Object%20Reference)))

(event EventTick
  (params (DeltaSeconds :type Float%20%28single-precision%29)))

(fn ConstructionScript)