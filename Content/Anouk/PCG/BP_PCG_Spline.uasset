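; BP_PCG_Spline is a PCG helper Blueprint that measures the X-axis length of a level segment between its LevelBegin and LevelEnd components.
; GetLevelOffsetValue stores the difference of their relative X locations in LevelTransformDifference, zeroing Y and Z, and prints a debug message.
; It runs in the Construction Script and again on BeginPlay.
; DisableMeshCollisions is an empty event, and the PCG reference in the event graph is unused.
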(event Custom|DisableMeshCollisions)

(event EventBeginPlay
  (CallFunction|GetLevelOffsetValue))

(event Collision|EventActorBeginOverlap
  (params (OtherActor :type Actor%20Object%20Reference)))

(event EventTick
  (params (DeltaSeconds :type Float%20%28single-precision%29)))

(fn ConstructionScript
  (CallFunction|GetLevelOffsetValue))

(fn GetLevelOffsetValue
  (Variables|Default|SetLevelTransformDifference (Math|Vector|MakeVector (- (.X (Math|Vector|BreakVector (Variables|/Script/Engine.SceneComponent|GetRelativeLocation (Variables|Default|GetLevelEnd)))) (.X (Math|Vector|BreakVector (Variables|/Script/Engine.SceneComponent|GetRelativeLocation (Variables|Default|GetLevelBegin))))) 0.0 0.0))
  (Development|PrintString "Get level offset" true true "(R=0.135633,G=0.006049,B=0.205079,A=1.000000)"))