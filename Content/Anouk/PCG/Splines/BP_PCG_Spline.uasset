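; Level segment actor with a spline-driven PCG component, providing randomized enemy spawn transforms and an X offset between level begin and end markers.
; Construction randomly nudges interior spline points in XY, keeping endpoints fixed, then regenerates the PCG.
; GetSplinePointTransforms turns spline points into spawn transforms with XY jitter, a hardcoded height lift and random yaw.
; Tick draws a debug label, set externally with an array index.
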(event Custom|SetDebugString
  (params (ArrayIndex :type Integer))
  (Variables|Default|SetDebugString (Utilities|String|Append (Utilities|GetDisplayName self) ": " (Utilities|String|ToString(Integer) ArrayIndex))))

(event EventBeginPlay
  (CallFunction|GetLevelOffsetValue))

(event Collision|EventActorBeginOverlap
  (params (OtherActor :type Actor%20Object%20Reference)))

(event EventTick
  (params (DeltaSeconds :type Float%20%28single-precision%29))
  (Rendering|Debug|DrawDebugString (Transformation|GetWorldLocation (Variables|Default|GetDefaultSceneRoot)) (Variables|Default|GetDebugString) 0 "(R=0.000000,G=0.521940,B=1.000000,A=1.000000)"))

(fn ConstructionScript
  (Development|PrintString (Utilities|String|Append (Utilities|GetDisplayName self) " construction script runs!") true true "(R=0.023674,G=0.541667,B=0.000000,A=1.000000)" 5.0)
  (CallFunction|RandomizeSplinePoints)
  (CallFunction|GetLevelOffsetValue))

(fn GetLevelOffsetValue
  (Variables|Default|SetLevelTransformDifference (Math|Vector|MakeVector (- (.X (Math|Vector|BreakVector (Variables|/Script/Engine.SceneComponent|GetRelativeLocation (Variables|Default|GetLevelEnd)))) (.X (Math|Vector|BreakVector (Variables|/Script/Engine.SceneComponent|GetRelativeLocation (Variables|Default|GetLevelBegin))))) 0.0 0.0))
  (Development|PrintString "Get level offset" true true "(R=0.135633,G=0.006049,B=0.205079,A=1.000000)"))

(fn GetSplinePointTransforms
  (params (Spline :type Spline%20Component%20Object%20Reference) (SplinePointNumber :type Integer))
  (Utilities|Array|Clear (Variables|Default|GetSplineTransforms))
  (for _index (range 0 (- SplinePointNumber 1))
    (bind _randomlocation (CallFunction|GetRandomEnemySpawnPosition (.location (Spline|GetTransformatSplinePoint Spline _index "World" false))))
    (Utilities|Array|Add (Variables|Default|GetSplineTransforms) (Math|Transform|MakeTransform (+ _randomlocation "0.000000,0.000000,90.000000") (Math|Rotator|MakeRotator (.Roll (Math|Rotator|BreakRotator (.rotation (Spline|GetTransformatSplinePoint Spline _index "World" false)))) (.Pitch (Math|Rotator|BreakRotator (.rotation (Spline|GetTransformatSplinePoint Spline _index "World" false)))) (Math|Random|RandomFloatinRange 0.0 3.6e+02)) (.scale (Spline|GetTransformatSplinePoint Spline _index "World" false)))))
  (return (Variables|Default|GetSplineTransforms)))

(fn GetRandomEnemySpawnPosition
  (params (Origin :type Vector))
  (bind (_x _y _z) (Math|Vector|BreakVector Origin))
  (bind _xvariation (LocalVariables|GetXVariation))
  (bind _yvariation (LocalVariables|GetYVariation))
  (return (Math|Vector|MakeVector (+ (Math|Random|RandomFloatinRange (* _xvariation -1.0) _xvariation) _x) (+ (Math|Random|RandomFloatinRange (* _yvariation -1.0) _yvariation) _y) _z)))

(fn RandomizeSplinePoints
  (bind _returnvalue (Math|Random|RandomUnitVector))
  (bind _spline (Variables|Default|GetSpline))
  (bind _pcg (Variables|Default|GetPCG))
  (bind _spline_2 (Variables|Default|GetSpline))
  (bind _returnvalue_2 (Spline|GetNumberOfSplinePoints _spline))
  (bind _returnvalue_3 (- _returnvalue_2 1))
  (Utilities|Array|Clear (LocalVariables|GetSplinePoints))
  (for _index (range 0 _returnvalue_3)
    (if (or (== _index 0) (== _index _returnvalue_3))
      (Utilities|Array|Add (LocalVariables|GetSplinePoints) (.location (Spline|GetTransformatSplinePoint _spline_2 _index "World" false)))
      (else
        (Utilities|Array|Add (LocalVariables|GetSplinePoints) (+ (.location (Spline|GetTransformatSplinePoint _spline_2 _index "World" false)) (* (Math|Vector|MakeVector (.x _returnvalue) (.y _returnvalue) 0.0) (LocalVariables|GetMultiplier))))
        (Spline|SetLocationatSplinePoint (Variables|Default|GetSpline) _index (+ (.location (Spline|GetTransformatSplinePoint _spline_2 _index "World" false)) (* (Math|Vector|MakeVector (.x _returnvalue) (.y _returnvalue) 0.0) (LocalVariables|GetMultiplier))) "World" true))))
  (Spline|SetSplinePoints _spline_2 (LocalVariables|GetSplinePoints) "World" true)
  (Class|PCGComponent|Cleanup _pcg true false)
  (PCG|Generate _pcg true))