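; Player controller Blueprint that toggles game pause from the IA_Pause input action.
; The action inverts the current paused state through SetPauseGame and prints a debug message.
; SetPauseGame shows or hides the mouse cursor to match, switching between Game And UI input when paused and Game Only when resumed.
; It creates no pause menu widget itself.
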(event Input|EnhancedActionEvents|EnhancedInputActionIA_Pause
  (params (ActionValue :type Boolean) (ElapsedSeconds :type Float%20%28double-precision%29) (TriggeredSeconds :type Float%20%28double-precision%29) (InputAction :type Input%20Action%20Object%20Reference :default "/Game/Anouk/GameStuff/IA_Pause.IA_Pause"))
  (CallFunction|SetPauseGame (not (Game|IsGamePaused)))
  (Development|PrintString "Game Pause Toggle"))

(event EventBeginPlay
  (Input|EnableInput 0))

(event EventTick
  (params (DeltaSeconds :type Float%20%28single-precision%29)))

(fn ConstructionScript)

(fn SetPauseGame
  (params (bPaused :type Boolean))
  (bind _returnvalue (Game|GetPlayerController 0))
  (bind _self self)
  (Input|EnableInput _self)
  (Variables|/Script/Engine.PlayerController|SetbShowMouseCursor _self bPaused)
  (if bPaused
    (Input|SetInputModeGameandUI _returnvalue 0 "DoNotLock" true false)
    (Game|SetGamePaused true)
    (else
      (Input|SetInputModeGameOnly _returnvalue false)
      (Game|SetGamePaused false))))