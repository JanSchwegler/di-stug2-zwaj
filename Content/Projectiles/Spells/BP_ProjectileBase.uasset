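; Base spell projectile that flies toward a target location at a set speed and reacts on impact.
; On BeginPlay it ignores its instigator or owner for collision, then aims its rotation and velocity at the target.
; A box hit calls OnProjectileImpact, spawns impact effect and sound, and destroys the actor.
; InitializeSpell packs scroll and rune data into a spell data struct.
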(event OnComponentHit(BoxCollision)
  (params (HitComponent :type Primitive%20Component%20Object%20Reference) (OtherActor :type Actor%20Object%20Reference) (OtherComp :type Primitive%20Component%20Object%20Reference) (NormalImpulse :type Vector :default "0, 0, 0") (Hit :type Hit%20Result%20Structure%20%28by%20ref%29))
  (bind _location (Collision|BreakHitResult Hit))
  (Default|CallOnProjectileImpact OtherActor Hit)
  (Niagara|SpawnSystematLocation (Variables|ScrollData|GetImpact%20Effect) _location)
  (Audio|PlaySoundatLocation (Variables|ScrollData|GetImpact%20Sound) _location "0, 0, 0" 1.0 1.0 0.0 0 0 0 0)
  (Actor|DestroyActor))

(event Custom|RotateToHitLocation
  (bind _returnvalue (Transformation|GetActorLocation))
  (bind _targetlocation (Variables|Target|GetTargetLocation))
  (bind _returnvalue_2 (Math|Rotator|FindLookatRotation _returnvalue _targetlocation))
  (Transformation|SetActorRotation _returnvalue_2)
  (Variables|/Script/Engine.MovementComponent|SetVelocity (Variables|Default|GetProjectileMovement) (* (Math|Vector|GetForwardVector _returnvalue_2) (Variables|ScrollData|GetSpeed))))

(event EventBeginPlay
  (bind _returnvalue (Game|GetInstigator))
  (Collision|IgnoreActorwhenMoving (Variables|Default|GetBoxCollision) (select (Utilities|IsValid _returnvalue) _returnvalue (Components|GetOwner)) true)
  (CallFunction|RotatetoHitLocation))

(event Collision|EventActorBeginOverlap
  (params (OtherActor :type Actor%20Object%20Reference)))

(fn ConstructionScript
  (bind _projectilemovement (Variables|Default|GetProjectileMovement))
  (Variables|/Script/Engine.ProjectileMovementComponent|SetInitialSpeed _projectilemovement (Variables|ScrollData|GetSpeed))
  (Variables|/Script/Engine.ProjectileMovementComponent|SetMaxSpeed _projectilemovement (Variables|ScrollData|GetSpeed))
  (Variables|Target|GetTarget
    (:then)
    (:else)))

(fn InitializeSpell
  (params (ScrollData :type S%20Scroll%20Data%20Structure) (RuneData :type S%20Rune%20Data%20Structure))
  (bind _scrolltype (Utilities|Struct|BreakS_ScrollData ScrollData))
  (bind (_runetype _effectstrength _duration) (Utilities|Struct|BreakS_RuneData RuneData))
  (return (Utilities|Struct|MakeS_SpellData (Utilities|Name|EnumtoName _scrolltype) (Utilities|Name|EnumtoName _runetype) _runetype _duration _effectstrength _scrolltype)))